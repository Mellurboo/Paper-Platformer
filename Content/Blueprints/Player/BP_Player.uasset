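; Player character for a 2D flipbook side-scroller, with Enhanced Input run, jump and crouch, plus the player UI widget.
; Movement runs along X, flipping control yaw to face the direction of travel.
; Each tick, a priority-ordered state check on death, velocity and crouch picks the sprite's flipbook.
; Damage and healing adjust health; death, also triggerable by input, disables control and reopens Level 1 after a delay.
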(event Custom|Update%20Animations
  ;[0.7129 0.166 1] Animation Handler
  (Sprite|SetFlipbook (Variables|Default|GetSprite) (stale _animation))
  (bind _animation (CallFunction|ApplyPlayerState)))

(event Custom|PlayerDead
  ;[1 0.2238 0.09399] Player Death Logic
  (Variables|Default|SetisDead true)
  (Pawn|Components|CharacterMovement|DisableMovement (Variables|Character|GetCharacterMovement))
  (Input|DisableInput (Game|GetPlayerController 0))
  (Utilities|FlowControl|Delay (Variables|Default|GetPlayerDeathResetTime))
  (CallFunction|ResetPlayerLevel))

(event Custom|Take%20Damage
  (params (Damage :type Float%20%28double-precision%29))
  ;[1 0 0] Player Death Logic
  (bind _output_get (Variables|Default|SetPlayerHealth (- (Variables|Default|GetPlayerHealth) Damage)))
  (if (<= _output_get 0.0)
    (CallFunction|PlayerDead)))

(event Custom|Heal
  (params (Value :type Float%20%28double-precision%29))
  ;[0.7801 1 0.4004] Heal Player
  (Variables|Default|SetPlayerHealth (Math|Float|Clamp(Float) (+ Value (Variables|Default|GetPlayerHealth)))))

(event Input|EnhancedActionEvents|EnhancedInputActionIA_Movement
  (params (ActionValue :type Float%20%28double-precision%29) (ElapsedSeconds :type Float%20%28double-precision%29) (TriggeredSeconds :type Float%20%28double-precision%29) (InputAction :type Input%20Action%20Object%20Reference :default "/Game/Blueprints/Player/Input/IA_Movement.IA_Movement"))
  ;[0.2602 0.6012 1] Player Movement Logic
  (Pawn|Input|AddMovementInput "1.000000,0.000000,0.000000" ActionValue false)
  (Math|Float|CompareFloat ActionValue 0.0
    (:>
      (CallFunction|SetControllerRotation 0.0))
    (:<
      (CallFunction|SetControllerRotation 1.8e+02))))

(event Input|EnhancedActionEvents|EnhancedInputActionIA_Jump
  (params (ActionValue :type Boolean) (ElapsedSeconds :type Float%20%28double-precision%29) (TriggeredSeconds :type Float%20%28double-precision%29) (InputAction :type Input%20Action%20Object%20Reference :default "/Game/Blueprints/Player/Input/IA_Jump.IA_Jump"))
  ;[0.3222 1 0.5057] Jumping Logic
  (Character|Jump))

(event Input|EnhancedActionEvents|EnhancedInputActionIA_Crouch
  (params (ActionValue :type Boolean) (ElapsedSeconds :type Float%20%28double-precision%29) (TriggeredSeconds :type Float%20%28double-precision%29) (InputAction :type Input%20Action%20Object%20Reference :default "/Game/Blueprints/Player/Input/IA_Crouch.IA_Crouch"))
  ;[0.257 0.2402 1] crouching
  (:Started
    (Character|Crouch))
  (:Completed
    (Character|UnCrouch)))

(event Input|EnhancedActionEvents|EnhancedInputActionIA_Die
  (params (ActionValue :type Boolean) (ElapsedSeconds :type Float%20%28double-precision%29) (TriggeredSeconds :type Float%20%28double-precision%29) (InputAction :type Input%20Action%20Object%20Reference :default "/Game/Blueprints/Player/Input/IA_Die.IA_Die"))
  ;[1 0.2238 0.09399] Player Death Logic
  (CallFunction|PlayerDead))

(event EventBeginPlay
  ;[1 0 0.4701] Init
  (CallFunction|GetPlayerandMappingContext)
  (bind _returnvalue (UserInterface|CreateWidget "/Game/UI/WB_PlayerUI.WB_PlayerUI_C"))
  (UserInterface|Viewport|AddtoViewport _returnvalue 0))

(event EventOnLanded
  (params (Hit :type Hit%20Result%20Structure%20%28by%20ref%29))
  ;[0.3222 1 0.5057] Jumping Logic
  (Character|StopJumping)
  (Sprite|SetFlipbook (Variables|Default|GetSprite) "/Game/Sprites/Player/Idle/Idle.Idle"))

(event EventTick
  (params (DeltaSeconds :type Float%20%28single-precision%29))
  ;[0.2602 0.6012 1] Player Movement Logic
  (CallFunction|UpdateAnimations))

(fn ConstructionScript)

(fn GetPlayerandMappingContext
  (bind _asplayer_controller (Utilities|Casting|CastToPlayerController (Pawn|GetController))
    (:then
      (Input|AddMappingContext (PlayerController|LocalPlayerSubsystems|GetEnhancedInputLocalPlayerSubsystem _asplayer_controller) "/Game/Blueprints/Player/Input/MC_PlayerController.MC_PlayerController" 0 "(bIgnoreAllPressedKeysUntilRelease=True,bForceImmediately=False,bNotifyUserSettings=False)"))
    (:CastFailed
      (Development|PrintString "Failed at cast to player" true true "(R=1.000000,G=0.000000,B=0.058872,A=1.000000)"))))

(fn SetControllerRotation
  (params (Yaw :type Float%20%28double-precision%29))
  (Pawn|SetControlRotation (Pawn|GetController) (Math|Rotator|MakeRotator 0.0 0.0 Yaw)))

(fn IsinMotion
  (return (> (Math|Vector|VectorLengthXY (Transformation|GetVelocity)) 0.0)))

(fn AnimationStateMachine
  (params (isDead :type Boolean) (isJumping :type Boolean) (isFalling :type Boolean) (isMoving :type Boolean) (isCrouching :type Boolean))
  ;[0.8693 0.3543 1] state machine logic (order sensitive)
  (if isDead
    (Variables|Default|SetStates "NewEnumerator6")
    (elif isJumping
      (Variables|Default|SetStates "NewEnumerator2")
      (elif isFalling
        (Variables|Default|SetStates "NewEnumerator3")
        (elif isMoving
          (Variables|Default|SetStates "NewEnumerator1")
          (elif isCrouching
            (Variables|Default|SetStates "NewEnumerator4")
            (else
              (Variables|Default|SetStates "NewEnumerator0")))))))
  (return (Utilities|Select :Index (Variables|Default|GetStates) :NewEnumerator0 "/Game/Sprites/Player/Idle/Idle.Idle" :NewEnumerator1 "/Game/Sprites/Player/Running/Running.Running" :NewEnumerator2 "/Game/Sprites/Player/Jumping/Jumping.Jumping" :NewEnumerator3 "/Game/Sprites/Player/Jumping/Jumping.Jumping" :NewEnumerator4 "/Game/Sprites/Player/Crouching/Crouched.Crouched" :NewEnumerator6 "/Game/Sprites/Player/Dead/Dead.Dead")))

(fn IsJumping
  (bind _returnvalue (Transformation|GetVelocity))
  (bind _returnvalue_2 (> (.z _returnvalue) 0.0))
  (if _returnvalue_2
    _
    (else
      _))
  (return _returnvalue_2))

(fn IsFalling
  (bind _returnvalue (Transformation|GetVelocity))
  (bind _returnvalue_2 (< (.z _returnvalue) 0.0))
  (if _returnvalue_2
    _
    (else
      _))
  (return _returnvalue_2))

(fn ApplyPlayerState
  (bind _returnvalue (CallFunction|IsinMotion))
  (bind _isjumping (CallFunction|IsFalling))
  (bind _isjumping_2 (CallFunction|IsJumping))
  (bind _animation (CallFunction|AnimationStateMachine (Variables|Default|GetisDead) _isjumping_2 _isjumping _returnvalue (AI|Components|NavMovement|IsCrouching (Variables|Character|GetCharacterMovement))))
  (return _animation))

(fn ResetPlayerLevel
  (bind _asgamemode (Utilities|Casting|CastToLevelGamemode (Game|GetGameMode))
    (:then
      (Game|OpenLevel(byObjectReference) "/Game/Levels/Levels/L_Level1.L_Level1"))
    (:CastFailed
      (return _asgamemode))))