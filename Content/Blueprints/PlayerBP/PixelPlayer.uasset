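; Player character for a 2D side-scrolling platformer, with Enhanced Input movement, jumping, crouching and projectile fire, plus a HUD widget.
; Each tick, a priority-ordered state check on death, velocity and crouch selects the sprite flipbook.
; Damage and healing adjust health, and death disables collision and input before reloading the example map after a delay.
; Fire re-arms shortly after release, and timed invulnerability tints the sprite and toggles CanTakeDamage, which TakeDamage itself never checks.
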(event Custom|Update%20Animations
  ;[0.7129 0.166 1] Animation Handler
  (Sprite|SetFlipbook (Variables|Default|GetSprite) (stale _animation))
  (bind _animation (CallFunction|ApplyPlayerState)))

(event Custom|PlayerDead
  ;[1 0.2238 0.09399] Player Death Logic
  (Collision|SetCollisionEnabled (Variables|Collision|GetCapsuleComponent) "NoCollision")
  (Variables|PlayerParams|SetisDead true)
  (Pawn|Components|CharacterMovement|DisableMovement (Variables|Character|GetCharacterMovement))
  (Input|DisableInput (Game|GetPlayerController 0))
  (Utilities|FlowControl|Delay (Variables|Default|GetPlayerDeathResetTime))
  (CallFunction|ResetPlayerLevel))

(event Custom|Take%20Damage
  (params (Damage :type Float%20%28double-precision%29))
  ;[1 0 0] Player Death Logic
  (bind _output_get (Variables|Default|SetPlayerHealth (- (Variables|Default|GetPlayerHealth) Damage)))
  (if (<= _output_get 0.0)
    (CallFunction|PlayerDead)))

(event Custom|Heal
  (params (Value :type Float%20%28double-precision%29))
  ;[0.7801 1 0.4004] Heal Player
  (Variables|Default|SetPlayerHealth (Math|Float|Clamp(Float) (+ Value (Variables|Default|GetPlayerHealth)))))

(event Custom|SetInvulnerability
  ;[1 0.3569 0.6238] Damage Invulnerability
  (Variables|PlayerParams|SetcanTakeDamage false)
  (Sprite|SetSpriteColor (Variables|Default|GetSprite) "(R=0.786458,G=0.259026,B=0.313896,A=1.000000)")
  (Utilities|FlowControl|Delay (Variables|Default|GetInvulnerabilityDuration))
  (Variables|PlayerParams|SetcanTakeDamage true)
  (Sprite|SetSpriteColor (Variables|Default|GetSprite) "(R=1.000000,G=1.000000,B=1.000000,A=1.000000)"))

(event Input|EnhancedActionEvents|EnhancedInputActionPlayerMovement_IA
  (params (ActionValue :type Float%20%28double-precision%29) (ElapsedSeconds :type Float%20%28double-precision%29) (TriggeredSeconds :type Float%20%28double-precision%29) (InputAction :type Input%20Action%20Object%20Reference :default "/Game/Blueprints/PlayerBP/Input/PlayerMovement_IA.PlayerMovement_IA"))
  ;[0.2602 0.6012 1] Player Movement Logic
  (Pawn|Input|AddMovementInput "1.000000,0.000000,0.000000" ActionValue false)
  (Math|Float|CompareFloat ActionValue 0.0
    (:>
      (CallFunction|SetControllerRotation 0.0))
    (:<
      (CallFunction|SetControllerRotation 1.8e+02))))

(event Input|EnhancedActionEvents|EnhancedInputActionCrouch_IA
  (params (ActionValue :type Boolean) (ElapsedSeconds :type Float%20%28double-precision%29) (TriggeredSeconds :type Float%20%28double-precision%29) (InputAction :type Input%20Action%20Object%20Reference :default "/Game/Blueprints/PlayerBP/Input/Crouch_IA.Crouch_IA"))
  ;[0.257 0.2402 1] crouching
  (:Started
    (Character|Crouch))
  (:Completed
    (Character|UnCrouch)))

(event Input|EnhancedActionEvents|EnhancedInputActionJumpInput_IA
  (params (ActionValue :type Boolean) (ElapsedSeconds :type Float%20%28double-precision%29) (TriggeredSeconds :type Float%20%28double-precision%29) (InputAction :type Input%20Action%20Object%20Reference :default "/Game/Blueprints/PlayerBP/Input/JumpInput_IA.JumpInput_IA"))
  ;[0.3222 1 0.5057] Jumping Logic
  (Character|Jump))

(event Input|EnhancedActionEvents|EnhancedInputActionFire_IA
  (params (ActionValue :type Boolean) (ElapsedSeconds :type Float%20%28double-precision%29) (TriggeredSeconds :type Float%20%28double-precision%29) (InputAction :type Input%20Action%20Object%20Reference :default "/Game/Blueprints/PlayerBP/Input/Fire_IA.Fire_IA"))
  ;[0.6193 0.2187 1] Fire Projectile
  (:Triggered
    (Utilities|FlowControl|DoOnce false :!label _label
      (:Completed
        (Game|SpawnActorfromClass "/Game/Blueprints/PlayerBP/BP_PlayerProjectile.BP_PlayerProjectile_C" (Transformation|GetWorldTransform (Variables|Default|GetProjectileOrigin)) "Undefined" "MultiplyWithRoot" 0 0))))
  (:Completed
    (Utilities|FlowControl|Delay 0.5)
    (goto _label Reset)))

(event EventBeginPlay
  ;[1 0 0.4701] Init
  (CallFunction|GetPlayerandMappingContext)
  (bind _returnvalue (UserInterface|CreateWidget "/Game/Blueprints/UI/BP_PlayerGUI_UI.BP_PlayerGUI_UI_C"))
  (bind _output_get (Variables|Default|SetPlayerGUI%20Reference _returnvalue))
  (UserInterface|Viewport|AddtoViewport _output_get 0)
  (Default|UpdateSlimeCount _output_get))

(event EventOnLanded
  (params (Hit :type Hit%20Result%20Structure%20%28by%20ref%29))
  ;[0.3222 1 0.5057] Jumping Logic
  (Character|StopJumping)
  (Sprite|SetFlipbook (Variables|Default|GetSprite) "/Game/Sprites/Player/Flipbooks/Idle/FB_Idle.FB_Idle"))

(event EventTick
  (params (DeltaSeconds :type Float%20%28single-precision%29))
  ;[0.2602 0.6012 1] Player Movement Logic
  (CallFunction|UpdateAnimations))

(fn ConstructionScript)

(fn GetPlayerandMappingContext
  (bind _asplayer_controller (Utilities|Casting|CastToPlayerController (Pawn|GetController)))
  (Input|AddMappingContext (PlayerController|LocalPlayerSubsystems|GetEnhancedInputLocalPlayerSubsystem _asplayer_controller) "/Game/Blueprints/PlayerBP/Input/PlayerContext_MC.PlayerContext_MC" 0 "(bIgnoreAllPressedKeysUntilRelease=True,bForceImmediately=False,bNotifyUserSettings=False)"))

(fn SetControllerRotation
  (params (Yaw :type Float%20%28double-precision%29))
  (Pawn|SetControlRotation (Pawn|GetController) (Math|Rotator|MakeRotator 0.0 0.0 Yaw)))

(fn IsinMotion
  (return (> (Math|Vector|VectorLengthXY (Transformation|GetVelocity)) 0.0)))

(fn AnimationStateMachine
  (params (isDead :type Boolean) (isJumping :type Boolean) (isFalling :type Boolean) (isMoving :type Boolean) (isCrouching :type Boolean))
  ;[0.8693 0.3543 1] state machine logic (order sensitive)
  (if isDead
    (Variables|PlayerParams|SetStates "NewEnumerator6")
    (elif isJumping
      (Variables|PlayerParams|SetStates "NewEnumerator2")
      (elif isFalling
        (Variables|PlayerParams|SetStates "NewEnumerator3")
        (elif isMoving
          (Variables|PlayerParams|SetStates "NewEnumerator1")
          (elif isCrouching
            (Variables|PlayerParams|SetStates "NewEnumerator4")
            (else
              (Variables|PlayerParams|SetStates "NewEnumerator0")))))))
  (return (Utilities|Select :Index (Variables|PlayerParams|GetStates) :NewEnumerator0 "/Game/Sprites/Player/Flipbooks/Idle/FB_Idle.FB_Idle" :NewEnumerator1 "/Game/Sprites/Player/Flipbooks/Running/FB_Running.FB_Running" :NewEnumerator2 "/Game/Sprites/Player/Flipbooks/Jumping/FB_Jumping.FB_Jumping" :NewEnumerator3 "/Game/Sprites/Player/Flipbooks/Jumping/FB_Jumping.FB_Jumping" :NewEnumerator4 "/Game/Sprites/Player/Flipbooks/Crouching/FB_Crouched.FB_Crouched" :NewEnumerator6 "/Game/Sprites/Player/Flipbooks/Dead/FB_Dead.FB_Dead")))

(fn IsJumping
  (bind _returnvalue (Transformation|GetVelocity))
  (bind _returnvalue_2 (> (.z _returnvalue) 0.0))
  (if _returnvalue_2
    _
    (else
      _))
  (return _returnvalue_2))

(fn IsFalling
  (bind _returnvalue (Transformation|GetVelocity))
  (bind _returnvalue_2 (< (.z _returnvalue) 0.0))
  (if _returnvalue_2
    _
    (else
      _))
  (return _returnvalue_2))

(fn ApplyPlayerState
  (bind _returnvalue (CallFunction|IsinMotion))
  (bind _isjumping (CallFunction|IsFalling))
  (bind _isjumping_2 (CallFunction|IsJumping))
  (bind _animation (CallFunction|AnimationStateMachine (Variables|PlayerParams|GetisDead) _isjumping_2 _isjumping _returnvalue (AI|Components|NavMovement|IsCrouching (Variables|Character|GetCharacterMovement))))
  (return _animation))

(fn ResetPlayerLevel
  (bind _asgm_platformer (Utilities|Casting|CastToGM_Platformer (Game|GetGameMode))
    (:then
      (Game|OpenLevel(byObjectReference) "/Game/Blueprints/Maps/2DSideScrollerExampleMap.2DSideScrollerExampleMap"))
    (:CastFailed
      (return _asgm_platformer))))