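; AntiPlayer is a 2D side-scroller enemy that walks horizontally, reversing whenever its capsule hits something, and knocks back and damages the PixelPlayer on contact.
; A looping timer line-traces forward and spawns BP_EnemyProjectile when it hits the player.
; Tick drives movement and selects flipbooks through a velocity-based state function.
; At zero health it disables collision and destroys itself after a delay; player-style input and level-reset helpers are never called here.
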(event OnComponentHit(CapsuleComponent)
  (params (HitComponent :type Primitive%20Component%20Object%20Reference) (OtherActor :type Actor%20Object%20Reference) (OtherComp :type Primitive%20Component%20Object%20Reference) (NormalImpulse :type Vector :default "0, 0, 0") (Hit :type Hit%20Result%20Structure%20%28by%20ref%29))
  ;[0.5837 0.5955 1] When the player touches the AI
  (if (not (Variables|Default|GetisDead))
    (Variables|AI|SetisMovingRight (not (Variables|AI|GetisMovingRight)))
    (bind _aspixel_player (Utilities|Casting|CastToPixelPlayer OtherActor))
    (bind _output_get (Variables|Default|SethitPixelPlayer _aspixel_player))
    (Character|LaunchCharacter _output_get (Math|Vector|MakeVector (select (Variables|AI|GetisMovingRight) 2.5e+02 -2.5e+02) 0.0 2.5e+02) true true)
    (if (Variables|/Game/Blueprints/PlayerBP/PixelPlayer.PixelPlayer_C|GetcanTakeDamage (Variables|Default|GethitPixelPlayer))
      (Default|SetInvulnerability (Variables|Default|GethitPixelPlayer))
      (Default|TakeDamage (Variables|Default|GethitPixelPlayer) (Variables|Default|GetDamage)))))

(event Custom|Update%20Animations
  ;[0.7129 0.166 1] Animation Handler
  (Sprite|SetFlipbook (Variables|Default|GetSprite) (stale _animation))
  (bind _animation (CallFunction|ApplyPlayerState)))

(event Custom|Take%20Damage
  (params (Damage :type Float%20%28double-precision%29))
  ;[1 0 0] Take Damage Event
  (bind _output_get (Variables|AI|SetHealth (- (Variables|AI|GetHealth) Damage)))
  (if (<= _output_get 0.0)
    (CallFunction|PlayerDead)
    (Utilities|FlowControl|Delay 4.0)
    (Actor|DestroyActor)))

(event Custom|Trace
  (bind _returnvalue (Transformation|GetActorLocation))
  ;[1 0.07997 0.3217] AI Tracing
  (bind _outhit (Collision|LineTraceByChannel _returnvalue (+ _returnvalue (* (Transformation|GetActorForwardVector) 500)) "TraceTypeQuery2" false 0 "None" true "(R=1.000000,G=0.000000,B=0.000000,A=1.000000)" "(R=0.000000,G=1.000000,B=0.000000,A=1.000000)" 2.0))
  (Utilities|Casting|CastToPixelPlayer (.HitActor (Collision|BreakHitResult _outhit)))
  (if (not (Variables|Default|GetisDead))
    (CallFunction|Shoot)))

(event Custom|Direction
  (bind _ismovingright (Variables|AI|GetisMovingRight))
  ;[1 0.3529 0.333] AI Movement Logic
  (Transformation|SetActorRotation (Math|Rotator|MakeRotator 0.0 0.0 (select _ismovingright 0.0 1.8e+02)))
  (Pawn|Input|AddMovementInput (select _ismovingright "1.000000,0.000000,0.000000" "-1.000000,0.000000,0.000000") 1.0 false))

(event Custom|Shoot
  ;[0.3623 1 0.5922] AI Shooting
  (Game|SpawnActorfromClass "/Game/Blueprints/EnemyBP/BP_EnemyProjectile.BP_EnemyProjectile_C" (Transformation|GetWorldTransform (Variables|Default|GetShootOrigin)) "Undefined" "MultiplyWithRoot" 0 0))

(event EventBeginPlay
  ;[1 0.07997 0.3217] AI Tracing
  (CallFunction|Trace)
  (Utilities|Time|SetTimerbyEvent (delegate Custom|Trace) 0.5 true))

(event EventTick
  (params (DeltaSeconds :type Float%20%28single-precision%29))
  ;[0.7635 0.3474 1] Movement calls
  (CallFunction|Direction)
  (CallFunction|UpdateAnimations))

(fn ConstructionScript)

(fn GetPlayerandMappingContext
  (bind _asplayer_controller (Utilities|Casting|CastToPlayerController (Pawn|GetController))
    (:then
      (Input|AddMappingContext (PlayerController|LocalPlayerSubsystems|GetEnhancedInputLocalPlayerSubsystem _asplayer_controller) 0 0 "(bIgnoreAllPressedKeysUntilRelease=True,bForceImmediately=False,bNotifyUserSettings=False)"))
    (:CastFailed
      (Development|PrintString "Failed at cast to player" true true "(R=1.000000,G=0.000000,B=0.058872,A=1.000000)"))))

(fn SetControllerRotation
  (params (Yaw :type Float%20%28double-precision%29))
  (Pawn|SetControlRotation (Pawn|GetController) (Math|Rotator|MakeRotator 0.0 0.0 Yaw)))

(fn IsinMotion
  (return (> (Math|Vector|VectorLengthXY (Transformation|GetVelocity)) 0.0)))

(fn AnimationStateMachine
  (params (isDead :type Boolean) (isJumping :type Boolean) (isFalling :type Boolean) (isMoving :type Boolean) (isCrouching :type Boolean))
  ;[0.8693 0.3543 1] state machine logic (order sensitive)
  (if isDead
    (Variables|Default|SetStates "NewEnumerator6")
    (elif isJumping
      (Variables|Default|SetStates "NewEnumerator2")
      (elif isFalling
        (Variables|Default|SetStates "NewEnumerator3")
        (elif isMoving
          (Variables|Default|SetStates "NewEnumerator1")
          (elif isCrouching
            (Variables|Default|SetStates "NewEnumerator4")
            (else
              (Variables|Default|SetStates "NewEnumerator0")))))))
  (return (Utilities|Select :Index (Variables|Default|GetStates) :NewEnumerator0 "/Game/Sprites/Player/Flipbooks/Idle/FB_Idle.FB_Idle" :NewEnumerator1 "/Game/Sprites/Player/Flipbooks/Running/FB_Running.FB_Running" :NewEnumerator2 "/Game/Sprites/Player/Flipbooks/Jumping/FB_Jumping.FB_Jumping" :NewEnumerator3 "/Game/Sprites/Player/Flipbooks/Jumping/FB_Jumping.FB_Jumping" :NewEnumerator4 "/Game/Sprites/Player/Flipbooks/Crouching/FB_Crouched.FB_Crouched" :NewEnumerator6 "/Game/Sprites/Player/Flipbooks/Dead/FB_Dead.FB_Dead")))

(fn IsJumping
  (bind _returnvalue (Transformation|GetVelocity))
  (bind _returnvalue_2 (> (.z _returnvalue) 0.0))
  (if _returnvalue_2
    _
    (else
      _))
  (return _returnvalue_2))

(fn IsFalling
  (bind _returnvalue (Transformation|GetVelocity))
  (bind _returnvalue_2 (< (.z _returnvalue) 0.0))
  (if _returnvalue_2
    _
    (else
      _))
  (return _returnvalue_2))

(fn ApplyPlayerState
  (bind _returnvalue (CallFunction|IsinMotion))
  (bind _isjumping (CallFunction|IsFalling))
  (bind _isjumping_2 (CallFunction|IsJumping))
  (bind _animation (CallFunction|AnimationStateMachine (Variables|Default|GetisDead) _isjumping_2 _isjumping _returnvalue (AI|Components|NavMovement|IsCrouching (Variables|Character|GetCharacterMovement))))
  (return _animation))

(fn ResetPlayerLevel
  (bind _asgm_platformer (Utilities|Casting|CastToGM_Platformer (Game|GetGameMode))
    (:then
      (Game|OpenLevel(byObjectReference) "/Game/Blueprints/Maps/2DSideScrollerExampleMap.2DSideScrollerExampleMap"))
    (:CastFailed
      (return _asgm_platformer))))

(fn PlayerDead
  (Collision|SetCollisionEnabled (Variables|Collision|GetCapsuleComponent) "NoCollision")
  (Variables|Default|SetisDead true))