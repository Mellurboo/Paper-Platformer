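; BP_SplineLift is a lift whose sprite travels along a spline, either automatically or on player contact.
; When IsTriggered is false the SplineMotionController timeline plays on BeginPlay; when true it plays once a PixelPlayer overlaps the Box.
; Each timeline update lerps its alpha over the spline length and sets LiftSprite's relative location from that local-space point, without sweeping.
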(event OnComponentBeginOverlap(Box)
  (params (OverlappedComponent :type Primitive%20Component%20Object%20Reference) (OtherActor :type Actor%20Object%20Reference) (OtherComp :type Primitive%20Component%20Object%20Reference) (OtherBodyIndex :type Integer) (bFromSweep :type Boolean) (SweepResult :type Hit%20Result%20Structure%20%28by%20ref%29))
  (bind _spline (Variables|Default|GetSpline))
  ;[0.3299 0 1] Check Trigger State (Entry Point)
  (Utilities|Casting|CastToPixelPlayer OtherActor)
  (if (== (Variables|Default|GetisTriggered) true)
    (bind _splinemotioncontroller (Timeline|SplineMotionController Play)
      (:Update
        (Transformation|SetRelativeLocation (Variables|Default|GetLiftSprite) (Spline|GetLocationatDistanceAlongSpline _spline (Math|Float|Lerp 0.0 (Spline|GetSplineLength _spline) _splinemotioncontroller) "Local") false false)))))

(event EventBeginPlay
  (bind _spline (Variables|Default|GetSpline))
  ;[0.3299 0 1] Check Trigger State (Entry Point)
  (if (== (Variables|Default|GetisTriggered) false)
    (bind _splinemotioncontroller (Timeline|SplineMotionController Play)
      (:Update
        (Transformation|SetRelativeLocation (Variables|Default|GetLiftSprite) (Spline|GetLocationatDistanceAlongSpline _spline (Math|Float|Lerp 0.0 (Spline|GetSplineLength _spline) _splinemotioncontroller) "Local") false false)))))

(fn ConstructionScript)